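; BP_DamageSphere is a short-lived sphere actor that destroys actors tagged "Wall" when it overlaps them.
; The Sphere component's begin overlap loops over the other actor's tags, destroys that actor on a match and prints any other tag.
; Tick increments a counter by one per frame and destroys the sphere once it reaches FinalTimeForDeath, so its lifetime depends on frame rate.
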(event OnComponentBeginOverlap(Sphere)
  (params (OverlappedComponent :type Primitive%20Component%20Object%20Reference) (OtherActor :type Actor%20Object%20Reference) (OtherComp :type Primitive%20Component%20Object%20Reference) (OtherBodyIndex :type Integer) (bFromSweep :type Boolean) (SweepResult :type Hit%20Result%20Structure%20%28by%20ref%29))
  (bind _array_element (Utilities|Array|ForEachLoopwithBreak (Variables|/Script/Engine.Actor|GetTags OtherActor))
    (:LoopBody
      (if (Utilities|Name|Equal(Name) _array_element "Wall")
        (Actor|DestroyActor OtherActor)
        (else
          (Development|PrintString (Utilities|String|ToString(Name) _array_element)))))))

(event EventBeginPlay)

(event Collision|EventActorBeginOverlap
  (params (OtherActor :type Actor%20Object%20Reference)))

(event EventTick
  (params (DeltaSeconds :type Float%20%28single-precision%29))
  (if (>= (Variables|Default|GetCurrentTimeForDeath) (Variables|Default|GetFinalTimeForDeath))
    (Actor|DestroyActor)
    (else
      (Variables|Default|SetCurrentTimeForDeath (+ (Variables|Default|GetCurrentTimeForDeath) 1.0)))))

(fn ConstructionScript)