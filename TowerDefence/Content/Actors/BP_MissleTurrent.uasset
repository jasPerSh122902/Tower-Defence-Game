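; Missile turret actor that turns toward a Wall actor and fires Bullet actors at regular intervals.
; Every Tick it looks up all Wall actors and snaps its rotation toward the first one, with no empty-list check.
; A counter rises by one per frame up to a limit, then resets as a Bullet spawns at the Gun component, so fire rate depends on frame rate.
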(event EventBeginPlay)

(event Collision|EventActorBeginOverlap
  (params (OtherActor :type Actor%20Object%20Reference)))

(event EventTick
  (params (DeltaSeconds :type Float%20%28single-precision%29))
  (bind _gun (Variables|Default|Getgun))
  (bind _outactors (Actor|GetAllActorsOfClass "/Game/Actors/Wall.Wall_C"))
  (Transformation|SetActorRotation (Math|Conversions|RotationFromXVector (- (Transformation|GetActorLocation (Utilities|Array|Get(acopy) _outactors)) (Transformation|GetActorLocation))))
  (if (>= (Variables|Default|GetcurrentShootTimer) (Variables|Default|GetLimitShootTimer))
    (Game|SpawnActorfromClass "/Game/Actors/Bullet.Bullet_C" (Math|Transform|MakeTransform (Transformation|GetWorldLocation _gun) (Transformation|GetWorldRotation _gun) "1,1,1") "Undefined" 0 0)
    (Variables|Default|SetcurrentShootTimer 0.0)
    (else
      (Variables|Default|SetcurrentShootTimer (+ (Variables|Default|GetcurrentShootTimer) 1.0)))))

(fn ConstructionScript)