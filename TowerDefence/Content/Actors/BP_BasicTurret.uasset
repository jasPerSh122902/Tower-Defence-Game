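; BP_BasicTurret is an auto-firing turret actor that turns toward BP_Enemy actors and shoots BP_Bullet from its Gun.
; Each Tick loops over all enemies and tracks a closest one using summed offset components rather than true distance.
; The stored value persists across frames, and farther enemies also set rotation, so the final facing follows the last enemy looped.
; A per-tick counter, independent of delta time, spawns a bullet upon reaching its limit, regardless of targets.
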(event EventBeginPlay)

(event Collision|EventActorBeginOverlap
  (params (OtherActor :type Actor%20Object%20Reference)))

(event EventTick
  (params (DeltaSeconds :type Float%20%28single-precision%29))
  (CallFunction|SetRotationMainBody)
  (CallFunction|SpawnBullet/SpawnCheck))

(fn ConstructionScript)

(fn SpawnBullet/SpawnCheck
  (bind _gun (Variables|Default|Getgun))
  (if (>= (Variables|Default|GetcurrentShootTimer) (Variables|Default|GetLimitShootTimer))
    (Game|SpawnActorfromClass "/Game/Actors/BP_Bullet.BP_Bullet_C" (Math|Transform|MakeTransform (Transformation|GetWorldLocation _gun) (Transformation|GetWorldRotation _gun) "1,1,1") "Undefined" 0 0)
    (Variables|Default|SetcurrentShootTimer 0.0)
    (else
      (Variables|Default|SetcurrentShootTimer (+ (Variables|Default|GetcurrentShootTimer) 1.0)))))

(fn SetRotationMainBody
  ;[1 1 1] Loop through the array of enemies and set the current enemy to the element that it is on.Set the current enemy direction
  (bind _outactors (Actor|GetAllActorsOfClass "/Game/Actors/BP_Enemy.BP_Enemy_C"))
  (for _array_element _outactors
    (bind _output_get (Variables|Default|SetcurrentEnemy (Transformation|GetActorLocation _array_element)))
    (bind _output_get_2 (Variables|Default|SetCurrentEnemyDirection (- _output_get (Transformation|GetActorLocation))))
    ;[1 1 1] Get the distance of current enemy and closes enemy
    (bind _output_get_3 (Variables|Default|SetDistanceOfCurrentEnemyToMe (+ (.x _output_get_2) (.y _output_get_2) (.z _output_get_2))))
    ;[1 1 1] Check to see if the current enemys distance is less than the closes enemy
    (if (< (Math|Float|Absolute(Float) _output_get_3) (Variables|Default|GetDistanceOfLastCheckEnemyToMe))
      ;[1 1 1] Set the ClosesEnemy to the current enemy
      (Variables|Default|SetDistanceOfLastCheckEnemyToMe (Variables|Default|GetDistanceOfCurrentEnemyToMe) :!label _label)
      (Variables|Default|SetClosesEnemy (Variables|Default|GetcurrentEnemy))
      (Variables|Default|SetCloasesEnemyDirection (Variables|Default|GetCurrentEnemyDirection))
      ;[1 1 1] Set the rotation to the closes enemy
      (Transformation|SetActorRotation (Math|Conversions|RotationFromXVector (Variables|Default|GetCloasesEnemyDirection)))
      (else
        ;[1 1 1] Check to see if the closes enemy was set by checking to see if it is 0 meaning it did not get a value yet
        (if (== (Variables|Default|GetDistanceOfLastCheckEnemyToMe) 0.0)
          (goto _label)
          (else
            ;[1 1 1] Set the rotation to the current enemy
            (Transformation|SetActorRotation (Math|Conversions|RotationFromXVector (Variables|Default|GetCurrentEnemyDirection)))))))))